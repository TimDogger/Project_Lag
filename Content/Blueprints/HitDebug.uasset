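; HitDebug is a debug actor that marks a hit with floating text and distinguishes server hits from other hits.
; On BeginPlay, IsServer selects the "SERVER HIT" or "HIT" label.
; Each tick it drifts upward, turns to face the first player's pawn, and draws a vertical debug line to world Z zero, red for server and blue otherwise.
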(event EventTick
  (params (DeltaSeconds :type Float%20%28single-precision%29))
  (bind _returnvalue (Transformation|GetActorLocation))
  (bind (_x _y) (Math|Vector|BreakVector _returnvalue))
  (Transformation|AddActorWorldOffset (Math|Vector|MakeVector 0.0 0.0 (* DeltaSeconds 1e+01)))
  (Transformation|SetActorRotation (Math|Rotator|FindLookatRotation (Transformation|GetActorLocation) (Transformation|GetActorLocation (Pawn|GetControlledPawn (Game|GetPlayerController 0)))))
  (Rendering|Debug|DrawDebugLine _returnvalue (Math|Vector|MakeVector _x _y 0.0) (Math|Color|SelectColor "(R=1.000000,G=0.000000,B=0.000000,A=1.000000)" "(R=0.000000,G=0.000000,B=1.000000,A=1.000000)" (Variables|Default|GetIsServer)) 0.0 0.0))

(event EventBeginPlay
  (Rendering|Components|TextRender|SetText (Variables|Default|GetTextRender) (select (Variables|Default|GetIsServer) (Utilities|Text|MakeLiteralText "SERVER HIT") (Utilities|Text|MakeLiteralText "HIT"))))

(fn ConstructionScript)