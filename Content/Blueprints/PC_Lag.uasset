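; PC_Lag is a player controller that creates the local player's on-screen UI.
; On BeginPlay it calls SetupUI only if it is the local controller.
; SetupUI creates the UI_Crosshair and UI_DebugInfo widgets with itself as owning player, stores each in a variable and adds both to the viewport.
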(event EventBeginPlay
  (Utilities|FlowControl|Sequence
    (:then_0
      ;[1 1 1] Local
      (if (Pawn|IsLocalController)
        (CallFunction|SetupUI)))))

(fn ConstructionScript)

(fn SetupUI
  (Utilities|FlowControl|Sequence
    (:then_0
      (bind _returnvalue (UserInterface|CreateWidget "/Game/UI/UI_Crosshair.UI_Crosshair_C" self))
      (bind _output_get (Variables|UI|SetCrosshair _returnvalue))
      (UserInterface|Viewport|AddtoViewport _output_get 0))
    (:then_1
      (bind _returnvalue_2 (UserInterface|CreateWidget "/Game/UI/UI_DebugInfo.UI_DebugInfo_C" self))
      (bind _output_get_2 (Variables|UI|SetDebugInfo _returnvalue_2))
      (UserInterface|Viewport|AddtoViewport _output_get_2 0))))