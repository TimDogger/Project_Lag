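; Playable character Blueprint for testing lag-compensated hitscan shooting, with debug visualization.
; The server fire trace has GM_Lag rewind all tracked actors by the shooter's latency, line-traces, damages any LagCharacter_Base hit, then restores positions.
; A separate client trace draws the shot from the first-person camera in the firing frame.
; Debug lines, HitDebug markers, damage messages and capsules on non-locally-controlled characters expose server results for comparison.
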(event Custom|Debug%20Draw%20Server%20Trace
  (params (Start :type Vector) (End :type Vector))
  ;[1 1 1] Отрисовка стрельбы на всех клиентах
  (Rendering|Debug|DrawDebugLine Start End "(R=1.000000,G=0.595663,B=0.000000,A=1.000000)" 5.0 1.0))

(event EventFireTraceInternal
  (params (AimDir :type Vector :default "0, 0, 0") (Location :type Vector :default "0, 0, 0") (Latency :type Float%20%28single-precision%29))
  (bind _returnvalue (* AimDir 1e+05))
  (bind _returnvalue_2 (+ Location _returnvalue))
  ;[1 1 1 1 50] SERVER TRACE.
  ;;[1 1 1] Отматываем всех отслеживаемых акторов на время, равное пингу стрелявшего
  (bind _asgm_lag (Utilities|Casting|CastToGM_Lag (Game|GetGameMode)))
  (Class|GMLag|RewindAllActors _asgm_lag Latency)
  ;;[1 1 1] Трассировка выстрела и отрисовка дебаг инфы
  (CallFunction|DebugDrawServerTrace Location _returnvalue_2)
  (bind _outhit (Collision|LineTraceByChannel Location _returnvalue_2 "TraceTypeQuery1" false 0 "ForDuration" true (Math|Color|SelectColor "(R=1.000000,G=0.000000,B=0.000000,A=1.000000)" "(R=0.000000,G=0.000000,B=1.000000,A=1.000000)" (Ability|HasAuthority))))
  (bind _aslag_character_base (Utilities|Casting|CastToLagCharacter_Base (.hitactor _outhit))
    (:then
      ;;;[1 1 1] Спавн актора, отрисовывающего Hit
      (Game|SpawnActorfromClass "/Game/Blueprints/HitDebug.HitDebug_C" (Math|Transform|MakeTransform (Math|Vector|MakeVector (.X (Math|Vector|BreakVector (.location _outhit))) (.Y (Math|Vector|BreakVector (.location _outhit))) 5e+02) "0, 0, 0" "1,1,1") "Undefined" 0 (Ability|HasAuthority) self)
      (Game|Damage|ApplyDamage _aslag_character_base 1.0 (Pawn|GetController) self "/Script/Engine.DamageType"))
    (:CastFailed
      _))
  ;;[1 1 1] Возвращаем всех отслеживаемых акторов в текущее положение
  (Class|GMLag|ForwardAllActors _asgm_lag))

(event EventClientFireTraceInternal
  (bind _firstpersoncameracomponent (Variables|Default|GetFirstPersonCameraComponent))
  (bind _returnvalue (Transformation|GetWorldLocation _firstpersoncameracomponent))
  ;[1 1 1] Трассировка стрельбы на клиенте. Вызывается в том же кадре когда клиент стреляет
  (Collision|LineTraceByChannel _returnvalue (+ _returnvalue (* (Math|Vector|GetForwardVector _firstpersoncameracomponent) 1e+05)) "TraceTypeQuery1" false 0 "ForDuration" true "(R=0.768712,G=1.000000,B=0.970067,A=1.000000)"))

(event EventTick
  (params (DeltaSeconds :type Float%20%28single-precision%29))
  (bind _capsulecomponent (Variables|Default|GetCapsuleComponent))
  (bind _returnvalue (Transformation|GetWorldTransform _capsulecomponent))
  ;[1 1 1] Отрисовка капсулы (кроме своей)
  (if (not (Pawn|IsLocallyControlled))
    (Rendering|Debug|DrawDebugCapsule (.location _returnvalue) (Components|Capsule|GetScaledCapsuleHalfHeight _capsulecomponent) (Components|Capsule|GetScaledCapsuleRadius _capsulecomponent) (.rotation _returnvalue) "(R=1.000000,G=1.000000,B=1.000000,A=1.000000)" 0.0 1.0)))

(event Game|Damage|EventAnyDamage
  (params (Damage :type Float%20%28single-precision%29) (DamageType :type Damage%20Type%20Object%20Reference) (InstigatedBy :type Controller%20Object%20Reference) (DamageCauser :type Actor%20Object%20Reference))
  ;[1 1 1] Вывод сообщения на сервере при фиксации попадания
  (Development|PrintText (Utilities|Text|FormatText "Player {1} dealed damage to {2}" InstigatedBy self) true true "(R=0.000000,G=0.660000,B=1.000000,A=1.000000)" 5.0))

(fn ConstructionScript)