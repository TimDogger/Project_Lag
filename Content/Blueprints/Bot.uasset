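; Bot is a simple AI pawn that walks back and forth between walls along its sideways axis.
; Each Tick it feeds a stored input vector into AddMovementInput.
; When its velocity is nearly zero, a FlipFlop switches that vector between the actor's right vector and its negation, so being stopped serves as the turn-around trigger without traces or collision events.
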(event EventTick
  (params (DeltaSeconds :type Float%20%28single-precision%29))
  (bind _returnvalue (Transformation|GetActorRightVector))
  ;[1 1 1] Простая ходьба пинг понгом между стенами
  (|CallParentFunction DeltaSeconds)
  (Utilities|FlowControl|Sequence
    (:then_0
      (if (Math|Vector|Equal(Vector) (Transformation|GetVelocity) "0, 0, 0" 0.001)
        (bind _isa (Utilities|FlowControl|FlipFlop)
          (:A
            _)
          (:B
            _))
        (Variables|Default|SetInputVector (Math|Vector|SelectVector (Math|Vector|NegateVector _returnvalue) _returnvalue _isa))))
    (:then_1
      (Pawn|Input|AddMovementInput (Variables|Default|GetInputVector) 1.0 false))))

(fn ConstructionScript
  (|CallParentFunction))