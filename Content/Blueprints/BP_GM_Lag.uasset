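; Game mode Blueprint (BP_GM_Lag) that provides a helper for spawning and possessing player pawns.
; SpawnPlayerPawn spawns PlayersPawnClass at the given transform's location with zero rotation and unit scale, owned by the controller.
; It stores the pawn in LocalPlayersPawn, has the controller possess it and returns it.
; PostLogin only calls the parent, and nothing in this Blueprint's graphs calls SpawnPlayerPawn.
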(event EventPostLogin
  (params (NewPlayer :type Player%20Controller%20Object%20Reference))
  (|CallParentFunction NewPlayer))

(fn ConstructionScript)

(fn SpawnPlayerPawn
  (params (NewPlayerController :type Controller%20Object%20Reference) (Transform :type Transform))
  (bind _returnvalue (Game|SpawnActorfromClass (Variables|Default|GetPlayersPawnClass) (Math|Transform|MakeTransform (.location Transform)) "Undefined" NewPlayerController 0))
  (LocalVariables|SetLocal_PlayersPawn _returnvalue)
  (Pawn|Possess NewPlayerController (LocalVariables|GetLocal_PlayersPawn))
  (return (LocalVariables|GetLocal_PlayersPawn)))